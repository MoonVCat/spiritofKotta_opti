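; Water actor (Agua) that switches the ThirdPersonCharacter between swimming and walking as it enters and leaves a Box.
; Overlap events react only to the character's Torso component, setting Swimming movement mode on entry and Walking on exit.
; Entry also changes FluidFriction on the character's current physics volume, which exit never restores.
; Both events set that volume's WaterVolume flag to false, so swimming relies on the explicit mode change.
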(event OnComponentBeginOverlap(Box)
  (params (OverlappedComponent :type Primitive%20Component%20Object%20Reference) (OtherActor :type Actor%20Object%20Reference) (OtherComp :type Primitive%20Component%20Object%20Reference) (OtherBodyIndex :type Integer) (bFromSweep :type Boolean) (SweepResult :type Hit%20Result%20Structure%20%28by%20ref%29))
  (bind _asthird_person_character (Utilities|Casting|CastToThirdPersonCharacter OtherActor))
  (if (== (Variables|/Game/ThirdPersonBP/Blueprints/ThirdPersonCharacter.ThirdPersonCharacter_C|GetTorso _asthird_person_character) OtherComp)
    (Variables|/Script/Engine.PhysicsVolume|SetbWaterVolume (Class|MovementComponent|GetPhysicsVolume (Variables|/Script/Engine.Character|GetCharacterMovement _asthird_person_character)) false)
    (Variables|/Script/Engine.PhysicsVolume|SetFluidFriction (Class|MovementComponent|GetPhysicsVolume (Variables|/Script/Engine.Character|GetCharacterMovement _asthird_person_character)) 0.8)
    (Pawn|Components|CharacterMovement|SetMovementMode (Variables|/Script/Engine.Character|GetCharacterMovement _asthird_person_character) "MOVE_Swimming" 0)))

(event OnComponentEndOverlap(Box)
  (params (OverlappedComponent :type Primitive%20Component%20Object%20Reference) (OtherActor :type Actor%20Object%20Reference) (OtherComp :type Primitive%20Component%20Object%20Reference) (OtherBodyIndex :type Integer))
  (bind _asthird_person_character (Utilities|Casting|CastToThirdPersonCharacter OtherActor))
  (if (== (Variables|/Game/ThirdPersonBP/Blueprints/ThirdPersonCharacter.ThirdPersonCharacter_C|GetTorso _asthird_person_character) OtherComp)
    (Variables|/Script/Engine.PhysicsVolume|SetbWaterVolume (Class|MovementComponent|GetPhysicsVolume (Variables|/Script/Engine.Character|GetCharacterMovement _asthird_person_character)) false)
    (Pawn|Components|CharacterMovement|SetMovementMode (Variables|/Script/Engine.Character|GetCharacterMovement _asthird_person_character) "MOVE_Walking" 0)))

(event EventBeginPlay)

(event Collision|EventActorBeginOverlap
  (params (OtherActor :type Actor%20Object%20Reference)))

(event EventTick
  (params (DeltaSeconds :type Float%20%28single-precision%29)))

(fn ConstructionScript)